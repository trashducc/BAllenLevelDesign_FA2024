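; Turret actor that sweeps its base in yaw and continuously fires ICA_Projectile_BP projectiles, starting at BeginPlay.
; The TurretMovement timeline drives rotation up to RotationAmt, looping at exactly 360 degrees and ping-ponging otherwise.
; A parallel Delay loop spawns projectiles at the Arrow and overrides their max speed.
; TurretAnimSpeed scales both timeline rate and fire rate, so faster turrets shoot more often.
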(event `self.ReceiveBeginPlay`
  ;[1 1 1] Sets speed for the animation timeline
  ;
  ; 1=normal; 2=twice as fast; 0.5 = twice as slow.
  (`TimelineComponent.SetPlayRate` (`self.TurretMovement`) (`self.TurretAnimSpeed`))
  (`|ExecutionSequence`
    (:`then_0`
      ;[1 1 1] Turret Rotation
      (bind (_direction _turretrotation) (`Timeline|TurretMovement` :!label _label)
        (:`Update`
          (`SceneComponent.K2_SetRelativeRotation` (`self.Base`) (`KismetMathLibrary.RLerp` (struct) (`KismetMathLibrary.MakeRotator` 0.0 0.0 (`self.RotationAmt`)) _turretrotation) false false))
        (:`Finished`
          (switch `ETimelineDirection` _direction
            (:`Forward`
              (if (== (`self.RotationAmt`) 360.0)
                (goto _label :!via `PlayFromStart`)
                (else
                  (goto _label :!via `Reverse`))))
            (:`Backward`
              (`TimelineComponent.SetPlayRate` (`self.TurretMovement`) (`self.TurretAnimSpeed`))
              (goto _label :!via `PlayFromStart`))))))
    (:`then_1`
      ;[1 1 1] Bullet Delay
      (bind _returnvalue (`|SpawnActorFromClass` "/Game/0_ICA/ICA10-25/ICA_Projectile_BP.ICA_Projectile_BP_C" (`SceneComponent.K2_GetComponentToWorld` (`self.Arrow`)) "Undefined" "MultiplyWithRoot" null null :!label _label_2))
      ;;[1 1 1] Sets Projectile Speed
      (set `ProjectileMovementComponent.MaxSpeed` (`self.ProjectileSpeed`) (`/Game/0_ICA/ICA10-25/ICA_Projectile_BP.ProjectileMovement` _returnvalue))
      (`KismetSystemLibrary.Delay` (/ (`self.ShootDelay`) (`self.TurretAnimSpeed`)))
      (goto _label_2))))

(fn `UserConstructionScript`)