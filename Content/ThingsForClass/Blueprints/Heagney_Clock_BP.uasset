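; Clock Blueprint that continuously animates a second hand in fixed six-degree steps from BeginPlay.
; UpdateRotators stores the RotatorSecond component's current relative rotation and a target six degrees lower in roll, then calls MoveClock.
; MoveClock plays the ClockMovement timeline to lerp between them, and its Finished pin calls UpdateRotators again, forming an endless loop.
; The graph moves only the second hand and never reads system time.
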(event `UpdateRotators`
  (bind _output_get (set `self.RotSecondBegin` (`SceneComponent.RelativeRotation` (`self.RotatorSecond`))))
  (set `self.RotSecondEnd` (`KismetMathLibrary.MakeRotator` (- (.roll _output_get) 6.0) (.pitch _output_get) (.yaw _output_get)))
  (`self.MoveClock`))

(event `self.ReceiveBeginPlay`
  (`self.UpdateRotators`))

(event `MoveClock`
  (bind (_direction _second) (`Timeline|ClockMovement` :!via `PlayFromStart`)
    (:`Update`
      (`SceneComponent.K2_SetRelativeRotation` (`self.RotatorSecond`) (`KismetMathLibrary.RLerp` (`self.RotSecondBegin`) (`self.RotSecondEnd`) _second) false false))
    (:`Finished`
      (`self.UpdateRotators`))))

(fn `UserConstructionScript`)