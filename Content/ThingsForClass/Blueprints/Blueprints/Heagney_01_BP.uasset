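; Trigger box actor that toggles the lamp mesh on the player's ThirdPersonLightCharacter between a lamppost and a smaller lamp.
; BeginPlay caches the cast character, and each player overlap alternates through a FlipFlop.
; Each side swaps materials, runs a timeline that stretches or squashes the mesh's Z scale, then swaps the static mesh when finished.
; Disconnected leftover nodes for gravity, walkable angle, mass and delays never run.
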(event `self.ReceiveBeginPlay`
  (bind _asthird_person_light_character (cast `/Game/ThirdPersonBP/Blueprints/ThirdPersonLightCharacter` (`GameplayStatics.GetPlayerCharacter` 0)))
  (set `self.Mylampy` _asthird_person_light_character))

(event `self.BoxCollision.OnComponentBeginOverlap`
  (params (OverlappedComponent :type "PrimitiveComponent Object Reference") (OtherActor :type "Actor Object Reference") (OtherComp :type "PrimitiveComponent Object Reference") (OtherBodyIndex :type Integer) (bFromSweep :type Boolean) (SweepResult :type "HitResult Structure (by ref)"))
  (bind _staticmesh (`/Game/ThirdPersonBP/Blueprints/ThirdPersonLightCharacter.StaticMesh` (`self.Mylampy`)))
  (bind _staticmesh_2 (`/Game/ThirdPersonBP/Blueprints/ThirdPersonLightCharacter.StaticMesh` (`self.Mylampy`)))
  (if (== OtherActor (`GameplayStatics.GetPlayerCharacter` 0))
    (`/Engine/EditorBlueprintResources/StandardMacros.FlipFlop`
      (:`A`
        (`|ExecutionSequence`
          (:`then_0`
            (`PrimitiveComponent.SetMaterial` _staticmesh_2 0 "/Game/ThingsForClass/Blueprints/StaticMesh/LampPost1.LampPost1")
            (`PrimitiveComponent.SetMaterial` _staticmesh_2 1 "/Game/ThingsForClass/Blueprints/StaticMesh/LampShade.LampShade")
            (`PrimitiveComponent.SetMaterial` _staticmesh_2 2 "/Game/ThingsForClass/Blueprints/StaticMesh/LampPost1.LampPost1"))
          (:`then_1`
            (bind (_direction _newtrack_1) (`Timeline|ScaleThingy`)
              (:`Update`
                (`SceneComponent.SetRelativeScale3D` _staticmesh_2 (`KismetMathLibrary.VLerp` (1.0 1.0 1.0) (1.0 1.0 7.0) _newtrack_1)))
              (:`Finished`
                (`StaticMeshComponent.SetStaticMesh` _staticmesh_2 "/Game/ThingsForClass/Blueprints/StaticMesh/lamppost.lamppost"))))))
      (:`B`
        (`|ExecutionSequence`
          (:`then_0`
            (`PrimitiveComponent.SetMaterial` _staticmesh 0 "/Game/ThingsForClass/Blueprints/StaticMesh/LampBase.LampBase")
            (`PrimitiveComponent.SetMaterial` _staticmesh 1 "/Game/ThingsForClass/Blueprints/StaticMesh/LampShade.LampShade")
            (`PrimitiveComponent.SetMaterial` _staticmesh 2 "/Game/ThingsForClass/Blueprints/StaticMesh/LampMetal.LampMetal"))
          (:`then_1`
            (bind (_direction_2 _newtrack_1_2) (`Timeline|Timeline`)
              (:`Update`
                (`SceneComponent.SetRelativeScale3D` _staticmesh (`KismetMathLibrary.VLerp` (1.0 1.0 1.0) (1.0 1.0 0.25) _newtrack_1_2)))
              (:`Finished`
                (`StaticMeshComponent.SetStaticMesh` _staticmesh "/Game/ThingsForClass/Blueprints/StaticMesh/lampy.lampy")))))))))

(fn `UserConstructionScript`)