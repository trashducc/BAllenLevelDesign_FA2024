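; Turret actor that continuously fires projectiles while animating the rotation of its base, starting at BeginPlay.
; A self-looping SpawnProjectile event spawns Projectile_BP at the Scene component's world transform, using a short delay between shots.
; In parallel, a timeline's RotateTurret track drives a rotator lerp toward a 360-degree turn on the Base, restarting after a brief pause.
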(event `self.ReceiveBeginPlay`
  (`self.SpawnProjectile`)
  (bind (_direction _rotateturret) (`Timeline|Timeline` :!label _label)
    (:`Update`
      (`SceneComponent.K2_SetRelativeRotation` (`self.Base`) (`KismetMathLibrary.RLerp` (struct) (struct :`Yaw` 360.0) _rotateturret) false false))
    (:`Finished`
      (`KismetSystemLibrary.Delay` 0.1)
      (goto _label :!via `PlayFromStart`))))

(event `SpawnProjectile`
  (`|SpawnActorFromClass` "/Game/Turret/Projectile_BP.Projectile_BP_C" (`SceneComponent.K2_GetComponentToWorld` (`self.Scene`)) "Undefined" "MultiplyWithRoot" null null :!label _label_2)
  (`KismetSystemLibrary.Delay` 0.1)
  (goto _label_2))

(fn `UserConstructionScript`)