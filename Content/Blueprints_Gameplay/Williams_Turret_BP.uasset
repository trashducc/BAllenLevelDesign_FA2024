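; Turret actor that sweeps its base in yaw while continuously spawning Williams_Projectile_BP from its Scene component at a fixed short interval.
; A timeline lerps the base up to TurretRotation at a TurretSpeed play rate, looping for a 360-degree rotation and ping-ponging otherwise.
; Each time the player character enters the Box, TurretSpeed triples cumulatively, speeding up the rotation but not the fire rate.
; The increaseSpeed event is an empty stub.
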(event `self.ReceiveBeginPlay`
  (`TimelineComponent.SetPlayRate` (`self.Turret Movement`) (`self.TurretSpeed`))
  (`|ExecutionSequence`
    (:`then_0`
      (bind (_direction _rotate_turret) (`Timeline|Turret Movement` :!label _label)
        (:`Update`
          (`SceneComponent.K2_SetRelativeRotation` (`self.Base`) (`KismetMathLibrary.RLerp` (struct) (`KismetMathLibrary.MakeRotator` 0.0 0.0 (`self.TurretRotation`)) _rotate_turret) false false))
        (:`Finished`
          (`TimelineComponent.SetPlayRate` (`self.Turret Movement`) (`self.TurretSpeed`))
          (if (== (`self.TurretRotation`) 360.0)
            (goto _label :!via `PlayFromStart`)
            (else
              (switch `ETimelineDirection` _direction
                (:`Forward`
                  (goto _label :!via `ReverseFromEnd`))
                (:`Backward`
                  (goto _label :!via `PlayFromStart`))))))))
    (:`then_1`
      (`|SpawnActorFromClass` "/Game/Blueprints_Gameplay/Williams_Projectile_BP.Williams_Projectile_BP_C" (`SceneComponent.K2_GetComponentToWorld` (`self.Scene`)) "Undefined" "MultiplyWithRoot" null null :!label _label_2)
      (`KismetSystemLibrary.Delay` 0.1)
      (goto _label_2))))

(event `self.Box.OnComponentBeginOverlap`
  (params (OverlappedComponent :type "PrimitiveComponent Object Reference") (OtherActor :type "Actor Object Reference") (OtherComp :type "PrimitiveComponent Object Reference") (OtherBodyIndex :type Integer) (bFromSweep :type Boolean) (SweepResult :type "HitResult Structure (by ref)"))
  (bind _turretspeed (`self.TurretSpeed`))
  (if (== OtherActor (`GameplayStatics.GetPlayerCharacter` 0))
    (set `self.TurretSpeed` (* _turretspeed 3.0))
    (`TimelineComponent.SetPlayRate` (`self.Turret Movement`) _turretspeed)))

(event `increaseSpeed`)

(fn `UserConstructionScript`)