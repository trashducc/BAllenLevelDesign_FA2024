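; Turret actor that spins continuously while firing projectiles at a fixed interval.
; On BeginPlay it starts an endless delay loop that spawns Heenan_Projectile_BP at the Scene component's world transform.
; The TurrentMovement timeline drives a rotator lerp through a full turn on the Base component, then restarts after a brief pause.
; Firing runs independently of rotation, with no targeting or stop condition.
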(event `Spawn Projectile`
  (`|SpawnActorFromClass` "/Game/Blueprints_Gameplay/Heenan_Projectile_BP.Heenan_Projectile_BP_C" (`SceneComponent.K2_GetComponentToWorld` (`self.Scene`)) "Undefined" "MultiplyWithRoot" null null :!label _label)
  (`KismetSystemLibrary.Delay` 0.2)
  (goto _label))

(event `self.ReceiveBeginPlay`
  ;[0.9626 0.03552 1 1 20] Rotates Turret
  (`self.Spawn Projectile`)
  (bind (_direction _rotate_turret) (`Timeline|Turrent Movement` :!label _label_2)
    (:`Update`
      (`SceneComponent.K2_SetRelativeRotation` (`self.Base`) (`KismetMathLibrary.RLerp` (struct) (struct :`Yaw` 360.0) _rotate_turret) false false))
    (:`Finished`
      (`KismetSystemLibrary.Delay` 0.1)
      (goto _label_2 :!via `PlayFromStart`))))

(fn `UserConstructionScript`)