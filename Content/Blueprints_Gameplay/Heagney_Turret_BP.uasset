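; Turret actor that spins continuously and fires projectiles on its own from BeginPlay, with no targeting or trigger.
; A timeline drives the Base component's relative rotation through a full turn and replays after a very brief delay when finished.
; In parallel, a custom event loops on a short delay, spawning Heagney_Projectile_BP at the Scene component's world transform.
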(event `self.ReceiveBeginPlay`
  (`self.SpawnProjectile`)
  (bind (_direction _rotate_turret) (`Timeline|TurretMovement` :!label _label)
    (:`Update`
      (`SceneComponent.K2_SetRelativeRotation` (`self.Base`) (`KismetMathLibrary.RLerp` (struct) (struct :`Yaw` 360.0) _rotate_turret) false false))
    (:`Finished`
      (`KismetSystemLibrary.Delay` 0.01)
      (goto _label :!via `PlayFromStart`))))

(event `SpawnProjectile`
  (`|SpawnActorFromClass` "/Game/Blueprints_Gameplay/Heagney_Projectile_BP.Heagney_Projectile_BP_C" (`SceneComponent.K2_GetComponentToWorld` (`self.Scene`)) "Undefined" "MultiplyWithRoot" null null :!label _label_2)
  (`KismetSystemLibrary.Delay` 0.2)
  (goto _label_2))

(fn `UserConstructionScript`)